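; Health pickup Blueprint that restores health to the player who picks it up.
; ItemPickup adds HealthIncrease to the player's current health, clamped between zero and HealthMax, and returns true.
; A player already at full health is left unchanged and the function returns false.
; The construction script only calls its parent, with no setup of its own.
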(fn ConstructionScript
  (|CallParentFunction))

(fn ItemPickup
  (params (Player :type First%20Person%20Character%20Base%20Object%20Reference))
  (if (< (Variables|/Script/MovementProject.FirstPersonCharacter|GethealthCurrent Player) (Variables|/Script/MovementProject.FirstPersonCharacter|GethealthMax Player))
    (Variables|/Script/MovementProject.FirstPersonCharacter|SethealthCurrent Player (Math|Float|Clamp(Float) (+ (Variables|/Script/MovementProject.FirstPersonCharacter|GethealthCurrent Player) (Variables|Default|GetHealthIncrease)) 0.0 (Variables|/Script/MovementProject.FirstPersonCharacter|GethealthMax Player)))
    (return true)
    (else
      (return false))))