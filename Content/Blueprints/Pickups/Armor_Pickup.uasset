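; Armor pickup Blueprint that restores a player's current armor by a set increase, clamped between zero and the player's maximum.
; The ItemPickup function applies the increase only when armor is below maximum and returns whether it did.
; A separate PickupEvent applies the same clamped increase without that check or return value.
; The construction script only calls its parent, so the class adds no setup there.
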(event EventPickupEvent
  (params (Player :type First%20Person%20Character%20Base%20Object%20Reference))
  (Variables|/Script/MovementProject.FirstPersonCharacter|SetarmorCurrent Player (Math|Float|Clamp(Float) (+ (Variables|/Script/MovementProject.FirstPersonCharacter|GetarmorCurrent Player) (Variables|Default|GetArmorIncrease)) 0.0 (Variables|/Script/MovementProject.FirstPersonCharacter|GetarmorMax Player))))

(fn ConstructionScript
  (|CallParentFunction))

(fn ItemPickup
  (params (Player :type First%20Person%20Character%20Base%20Object%20Reference))
  (if (< (Variables|/Script/MovementProject.FirstPersonCharacter|GetarmorCurrent Player) (Variables|/Script/MovementProject.FirstPersonCharacter|GetarmorMax Player))
    (Variables|/Script/MovementProject.FirstPersonCharacter|SetarmorCurrent Player (Math|Float|Clamp(Float) (+ (Variables|/Script/MovementProject.FirstPersonCharacter|GetarmorCurrent Player) (Variables|Default|GetArmorIncrease)) 0.0 (Variables|/Script/MovementProject.FirstPersonCharacter|GetarmorMax Player)))
    (return true)
    (else
      (return false))))