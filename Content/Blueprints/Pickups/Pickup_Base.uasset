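; Base pickup actor that a player-controlled first-person character collects by overlapping it.
; On overlap it prints a debug message, checks the other actor's class and control, then passes the character to ItemPickup and destroys itself if that returns true.
; ItemPickup returns false here and PickupEvent is empty, so the base alone is never consumed and both act as stubs.
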(event Custom|PickupEvent
  (params (Player :type First%20Person%20Character%20Base%20Object%20Reference)))

(event Collision|EventActorBeginOverlap
  (params (OtherActor :type Actor%20Object%20Reference))
  (bind _asfirst_person_character_base (Utilities|Casting|CastToFirstPersonCharacter_Base OtherActor))
  (Development|PrintString "Hello")
  (if (and (Utilities|ClassIsChildOf (Utilities|GetClass OtherActor) "/Script/MovementProject.FirstPersonCharacter") (Pawn|IsPlayerControlled _asfirst_person_character_base))
    (bind _pickedup_ (CallFunction|ItemPickup _asfirst_person_character_base))
    (if _pickedup_
      (Actor|DestroyActor))))

(fn ConstructionScript)

(fn ItemPickup
  (params (Player :type First%20Person%20Character%20Base%20Object%20Reference))
  (return false))