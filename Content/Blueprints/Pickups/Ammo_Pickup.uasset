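; Ammo pickup that refills the current ammo of the weapon the player is carrying.
; ItemPickup casts the player's Weapon child actor to Weapon_Base and, if it is below max, adds AmmoIncrease clamped between zero and AmmoMax.
; It returns true only when ammo is added and false when the weapon is already full.
; The construction script only calls its parent.
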(fn ConstructionScript
  (|CallParentFunction))

(fn ItemPickup
  (params (Player :type First%20Person%20Character%20Base%20Object%20Reference))
  (bind _weapon (Variables|/Game/Blueprints/Player/FirstPersonCharacter_Base.FirstPersonCharacter_Base_C|GetWeapon Player))
  (bind _childactor (Variables|/Script/Engine.ChildActorComponent|GetChildActor _weapon))
  (bind _weapon_2 (Variables|/Game/Blueprints/Player/FirstPersonCharacter_Base.FirstPersonCharacter_Base_C|GetWeapon Player))
  (bind _asweapon_base (Utilities|Casting|CastToWeapon_Base _childactor))
  (bind _childactor_2 (Variables|/Script/Engine.ChildActorComponent|GetChildActor _weapon_2))
  (bind _asweapon_base_2 (Utilities|Casting|CastToWeapon_Base _childactor_2))
  (if (< (Variables|/Script/MovementProject.Weapon|GetammoCurrent _asweapon_base) (Variables|/Script/MovementProject.Weapon|GetammoMax _asweapon_base))
    (Variables|/Script/MovementProject.Weapon|SetammoCurrent _asweapon_base_2 (Math|Integer|Clamp(Integer) (+ (Variables|/Script/MovementProject.Weapon|GetammoCurrent _asweapon_base_2) (Variables|Default|GetAmmoIncrease)) 0 (Variables|/Script/MovementProject.Weapon|GetammoMax _asweapon_base_2)))
    (return true)
    (else
      (return false))))