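; Speed perk Blueprint that raises the player's walk and sprint speeds across three tiers.
; SetDefaultValues caches the player's base walk and sprint speeds.
; Each tier event multiplies those cached bases by its own multiplier, writing to the character movement's MaxWalkSpeed and the player's Speed and SprintSpeed, so tiers do not compound.
; RemoveEffects restores the cached base values.
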(event EventTier1
  (bind _player (Variables|Default|GetPlayer))
  (bind _output_get (Variables|/Script/Engine.CharacterMovementComponent|SetMaxWalkSpeed (Variables|/Script/Engine.Character|GetCharacterMovement (Variables|Default|GetPlayer)) (* (Variables|Default|GetBaseWalkSpeed) (Variables|Default|GetTier1Multiplier))))
  (Variables|/Script/MovementProject.FirstPersonCharacter|Setspeed _player _output_get)
  (Variables|/Script/MovementProject.FirstPersonCharacter|SetsprintSpeed _player (* (Variables|Default|GetBaseSprintSpeed) (Variables|Default|GetTier1Multiplier))))

(event EventTier2
  (bind _player (Variables|Default|GetPlayer))
  (bind _output_get (Variables|/Script/Engine.CharacterMovementComponent|SetMaxWalkSpeed (Variables|/Script/Engine.Character|GetCharacterMovement (Variables|Default|GetPlayer)) (* (Variables|Default|GetBaseWalkSpeed) (Variables|Default|GetTier2Multiplier))))
  (Variables|/Script/MovementProject.FirstPersonCharacter|Setspeed _player _output_get)
  (Variables|/Script/MovementProject.FirstPersonCharacter|SetsprintSpeed _player (* (Variables|Default|GetBaseSprintSpeed) (Variables|Default|GetTier2Multiplier))))

(event EventTier3
  (bind _player (Variables|Default|GetPlayer))
  (bind _output_get (Variables|/Script/Engine.CharacterMovementComponent|SetMaxWalkSpeed (Variables|/Script/Engine.Character|GetCharacterMovement (Variables|Default|GetPlayer)) (* (Variables|Default|GetBaseWalkSpeed) (Variables|Default|GetTiier3Multiplier))))
  (Variables|/Script/MovementProject.FirstPersonCharacter|Setspeed _player _output_get)
  (Variables|/Script/MovementProject.FirstPersonCharacter|SetsprintSpeed _player (* (Variables|Default|GetBaseSprintSpeed) (Variables|Default|GetTiier3Multiplier))))

(event EventRemoveEffects
  (bind _player (Variables|Default|GetPlayer))
  (bind _output_get (Variables|/Script/Engine.CharacterMovementComponent|SetMaxWalkSpeed (Variables|/Script/Engine.Character|GetCharacterMovement (Variables|Default|GetPlayer)) (Variables|Default|GetBaseWalkSpeed)))
  (Variables|/Script/MovementProject.FirstPersonCharacter|Setspeed _player _output_get)
  (Variables|/Script/MovementProject.FirstPersonCharacter|SetsprintSpeed _player (Variables|Default|GetBaseSprintSpeed)))

(event EventSetDefaultValues
  (bind _player (Variables|Default|GetPlayer))
  (Variables|Default|SetBaseWalkSpeed (Variables|/Script/MovementProject.FirstPersonCharacter|Getspeed _player))
  (Variables|Default|SetBaseSprintSpeed (Variables|/Script/MovementProject.FirstPersonCharacter|GetsprintSpeed _player)))

(fn ConstructionScript
  (|CallParentFunction))