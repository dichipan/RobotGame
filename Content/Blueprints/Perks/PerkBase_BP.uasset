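; Base Blueprint for tiered player perks, with empty events for child perks to define default, per-tier and restore behavior.
; On BeginPlay it adds an icon widget to the player's HUD.
; Upgrades and downgrades update the player body, linked machine and tier text, then fire the matching tier event.
; Dropping to tier zero queues the perk for removal, while RemovePerk restores defaults, unregisters it and destroys the actor.
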(event Custom|Tier%201)

(event Custom|Tier%202)

(event Custom|Tier%203)

(event Custom|Remove%20Perk
  (bind _player (Variables|Default|GetPlayer))
  (CallFunction|RestoreDefaultValues)
  (Utilities|Array|RemoveItem (Variables|/Game/Blueprints/Player/FirstPersonCharacter_Base.FirstPersonCharacter_Base_C|GetPerks _player) self)
  (Default|RemovePerk (Variables|/Game/Blueprints/Player/FirstPersonCharacter_Base.FirstPersonCharacter_Base_C|GetHUDWidget _player) (Variables|Default|GetPerkWidget))
  (Actor|DestroyActor))

(event Custom|UpgradePerk
  (bind _result (Math|Integer|IncrementInt (Variables|Default|GetTier))
    (:%20%20
      (Default|UpdateBody (Variables|Default|GetPlayer))
      (CallFunction|UpdateMachine)
      (CallFunction|UpdateWidget)
      (switch int _result
        (:1
          (CallFunction|Tier1))
        (:2
          (CallFunction|Tier2))
        (:3
          (CallFunction|Tier3))))))

(event Custom|DowngradePerk
  (bind _result (Math|Integer|DecrementInt (Variables|Default|GetTier))
    (:%20%20
      (Default|UpdateBody (Variables|Default|GetPlayer))
      (CallFunction|UpdateMachine)
      (CallFunction|UpdateWidget)
      (switch int _result
        (:0
          (CallFunction|AddtoRemoveQueue))
        (:1
          (CallFunction|Tier1))
        (:2
          (CallFunction|Tier2))))))

(event Custom|Restore%20Default%20Values)

(event Custom|Set%20Default%20Values)

(event Custom|AddToRemoveQueue
  (Utilities|Array|Add (Variables|/Game/Blueprints/Player/FirstPersonCharacter_Base.FirstPersonCharacter_Base_C|GetPerksToRemove (Variables|Default|GetPlayer)) self))

(event EventBeginPlay
  (bind _returnvalue (UserInterface|CreateWidget "/Game/Blueprints/HUD/PerkBase_Widget.PerkBase_Widget_C"))
  (bind _output_get (Variables|Default|SetPerkWidget _returnvalue))
  (Variables|/Script/UMG.Image|SetBrush (Variables|/Game/Blueprints/HUD/PerkBase_Widget.PerkBase_Widget_C|GetPerkIcon _output_get) (Class|WidgetBlueprintLibrary|MakeBrushfromTexture (Variables|Default|GetPerkIcon) 100 100))
  (Default|AddPerk (Variables|/Game/Blueprints/Player/FirstPersonCharacter_Base.FirstPersonCharacter_Base_C|GetHUDWidget (Variables|Default|GetPlayer)) (Variables|Default|GetPerkWidget))
  (CallFunction|SetDefaultValues))

(fn ConstructionScript)

(fn UpdateMachine
  (Utilities|IsValid (Variables|Default|GetMachine)
    (:Is%20Valid
      (Variables|/Game/Blueprints/Perks/PerkMachine_BP.PerkMachine_BP_C|SetTier (Variables|Default|GetMachine) (Variables|Default|GetTier))
      (if (not (Utilities|Enum|Equal(Enum) (Variables|/Game/Blueprints/Player/FirstPersonCharacter_Base.FirstPersonCharacter_Base_C|GetHint (Variables|Default|GetPlayer)) ""))
        (Default|UpdateHint (Variables|Default|GetMachine) (Variables|Default|GetPlayer))))))

(fn UpdateWidget
  (Variables|/Script/UMG.TextBlock|SetText (Variables|/Game/Blueprints/HUD/PerkBase_Widget.PerkBase_Widget_C|GetPerkTier (Variables|Default|GetPerkWidget)) (Utilities|Text|ToText(Integer) (Variables|Default|GetTier))))