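; Perk machine that sells a player its configured perk class or upgrades the one they already own, in exchange for points.
; Interact requires the perk below tier three and BodyCurrent below BodyMax, then deducts the price for the machine's current Tier.
; A first purchase spawns a perk actor linked to machine and player, then upgrades it; later purchases upgrade that instance.
; Hint shows the tier's text and any non-zero price.
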(event Custom|UpdateHint
  (params (Player :type First%20Person%20Character%20Base%20Object%20Reference))
  (bind _tierprices (Variables|Default|GetTierPrices))
  (bind _tier (Variables|Default|GetTier))
  (bind _output (Utilities|Array|Get(acopy) _tierprices _tier))
  (Variables|/Game/Blueprints/Player/FirstPersonCharacter_Base.FirstPersonCharacter_Base_C|SetHint Player (Utilities|Array|Get(acopy) (Variables|Default|GetTierHints) (Variables|Default|GetTier)))
  (if (!= _output 0)
    (Variables|/Game/Blueprints/Player/FirstPersonCharacter_Base.FirstPersonCharacter_Base_C|SetHintPrice Player (Utilities|String|ToString(Integer) _output))))

(event EventInteractAction
  (params (Player :type First%20Person%20Character%20Base%20Object%20Reference))
  (bind _output_get (Variables|Default|SetPlayer Player))
  (Variables|Default|SetPerk 0)
  (bind _array_element (Utilities|Array|ForEachLoopwithBreak (Variables|/Game/Blueprints/Player/FirstPersonCharacter_Base.FirstPersonCharacter_Base_C|GetPerks _output_get) :!label _label)
    (:LoopBody
      (if (== (Utilities|GetClass _array_element) (Variables|Default|GetPerkClass))
        (Variables|Default|SetPerk _array_element)
        (goto _label Break)))
    (:Completed
      (Utilities|IsValid (Variables|Default|GetPerk)
        (:Is%20Valid
          (Default|UpgradePerk (Variables|Default|GetPerk)))
        (:Is%20Not%20Valid
          (bind _returnvalue (Game|SpawnActorfromClass (Variables|Default|GetPerkClass) (Math|Transform|MakeTransform "0, 0, 0" "0, 0, 0" "1.000000,1.000000,1.000000") "Undefined" "MultiplyWithRoot" 0 self (Variables|Default|GetPlayer) 0))
          (Utilities|Array|Add (Variables|/Game/Blueprints/Player/FirstPersonCharacter_Base.FirstPersonCharacter_Base_C|GetPerks (Variables|Default|GetPlayer)) _returnvalue)
          (Default|UpgradePerk _returnvalue))))))

(event EventInteract
  (params (Player :type First%20Person%20Character%20Base%20Object%20Reference))
  (bind _canupgrade_ (CallFunction|CanUpgrade? Player))
  (if _canupgrade_
    (bind _enoughpoints_ (CallFunction|SpendPoints Player))
    (if _enoughpoints_
      (CallFunction|InteractAction Player))))

(event EventHint
  (params (Player :type First%20Person%20Character%20Base%20Object%20Reference))
  (CallFunction|UpdateHint Player))

(fn ConstructionScript
  (|CallParentFunction))

(fn CanUpgrade?
  (params (Player :type First%20Person%20Character%20Base%20Object%20Reference))
  (for _array_element (Variables|/Game/Blueprints/Player/FirstPersonCharacter_Base.FirstPersonCharacter_Base_C|GetPerks Player)
    (if (and (== (Utilities|GetClass _array_element) (Variables|Default|GetPerkClass)) (>= (Variables|/Game/Blueprints/Perks/PerkBase_BP.PerkBase_BP_C|GetTier _array_element) 3))
      (LocalVariables|SetPerkUpgradeable? false)))
  (if (and (< (Variables|/Game/Blueprints/Player/FirstPersonCharacter_Base.FirstPersonCharacter_Base_C|GetBodyCurrent Player) (Variables|/Game/Blueprints/Player/FirstPersonCharacter_Base.FirstPersonCharacter_Base_C|GetBodyMax Player)) (LocalVariables|GetPerkUpgradeable?))
    (return true)
    (else
      (return false))))

(fn SpendPoints
  (params (Player :type First%20Person%20Character%20Base%20Object%20Reference))
  (bind _tierprices (Variables|Default|GetTierPrices))
  (bind _tier (Variables|Default|GetTier))
  (bind _output (Utilities|Array|Get(acopy) _tierprices _tier))
  (if (>= (Variables|/Script/MovementProject.FirstPersonCharacter|Getpoints Player) _output)
    (Class|FirstPersonCharacter|AddPoints Player (* _output -1))
    (return true)
    (else
      (return false))))