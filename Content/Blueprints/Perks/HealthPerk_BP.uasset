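; Health perk Blueprint that raises the player's maximum health across three tiers.
; It caches the player's starting max health as a base, and each tier event sets max health to that base plus a tier bonus, so tiers replace rather than stack.
; Every tier change, including removing the perk to restore the base, also refills current health to the new maximum.
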(event EventRemoveEffects
  (bind _player (Variables|Default|GetPlayer))
  (bind _output_get (Variables|/Script/MovementProject.FirstPersonCharacter|SethealthMax _player (Variables|Default|GetBaseHealth)))
  (Variables|/Script/MovementProject.FirstPersonCharacter|SethealthCurrent _player _output_get))

(event EventSetDefaultValues
  (Variables|Default|SetBaseHealth (Variables|/Script/MovementProject.FirstPersonCharacter|GethealthMax (Variables|Default|GetPlayer))))

(event EventTier1
  (bind _player (Variables|Default|GetPlayer))
  (bind _output_get (Variables|/Script/MovementProject.FirstPersonCharacter|SethealthMax _player (+ (Variables|Default|GetBaseHealth) (Variables|Default|GetTier1Health))))
  (Variables|/Script/MovementProject.FirstPersonCharacter|SethealthCurrent _player _output_get))

(event EventTier2
  (bind _player (Variables|Default|GetPlayer))
  (bind _output_get (Variables|/Script/MovementProject.FirstPersonCharacter|SethealthMax _player (+ (Variables|Default|GetBaseHealth) (Variables|Default|GetTier2Health))))
  (Variables|/Script/MovementProject.FirstPersonCharacter|SethealthCurrent _player _output_get))

(event EventTier3
  (bind _player (Variables|Default|GetPlayer))
  (bind _output_get (Variables|/Script/MovementProject.FirstPersonCharacter|SethealthMax _player (+ (Variables|Default|GetBaseHealth) (Variables|Default|GetTier3Health))))
  (Variables|/Script/MovementProject.FirstPersonCharacter|SethealthCurrent _player _output_get))

(fn ConstructionScript
  (|CallParentFunction))