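; Base Blueprint for projectile weapons that spawn a Projectile_Base when the owning player attacks.
; Attack checks magazine ammo and a CanAttack gate, then spends a round, calls Recoil and spawns the projectile at the muzzle, aimed along the player camera's rotation with damage and shooter passed in.
; A RateOfFire delay reopens the gate, and Attack calls itself again while a full-auto weapon's trigger is held.
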(event EventAttack
  (params (player :type First%20Person%20Character%20Object%20Reference))
  (Variables|Default|SetowningPlayer player)
  (if (and (> (Variables|Default|GetammoMagazineCurrent) 0) (Variables|Default|GetcanAttack))
    (Math|Integer|DecrementInt (Variables|Default|GetammoMagazineCurrent)
      (:%20%20
        (CallFunction|Recoil)
        (Variables|Default|SetcanAttack false)
        (Game|SpawnActorfromClass "/Game/Blueprints/Weapons/Projectile_Base.Projectile_Base_C" (Math|Transform|MakeTransform (Transformation|GetWorldLocation (Variables|Default|GetMuzzle)) (Transformation|GetWorldRotation (Variables|/Script/MovementProject.FirstPersonCharacter|GetplayerCamera (Variables|Default|GetowningPlayer))) "1.000000,1.000000,1.000000") "Undefined" "MultiplyWithRoot" 0 (Variables|Default|Getdamage) (Variables|Default|GetowningPlayer) 0)
        (Utilities|FlowControl|Delay (Variables|Default|GetrateOfFire))
        (Variables|Default|SetcanAttack true)
        (if (and (Variables|/Script/MovementProject.FirstPersonCharacter|GetholdingAttack (Variables|Default|GetowningPlayer)) (Variables|Default|GetFullAuto?))
          (Class|Weapon|Attack (Variables|Default|GetowningPlayer)))))))

(fn ConstructionScript
  (|CallParentFunction))