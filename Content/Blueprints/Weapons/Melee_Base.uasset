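; Base melee weapon Blueprint whose Attack event deals damage to whatever lies just in front of the attacking player's camera.
; A short multi sphere trace along the camera's forward vector ignores the owner, applies Damage to every hit result and draws debug shapes.
; A blocking hit plays a world camera shake at the camera, and a CanAttack flag reset after a RateOfFire delay gates repeat attacks.
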(event EventAttack
  (params (player :type First%20Person%20Character%20Object%20Reference))
  (Variables|Default|SetowningPlayer player)
  (if (Variables|Default|GetcanAttack)
    (Variables|Default|SetcanAttack false)
    (bind (_outhits _returnvalue) (Collision|MultiSphereTraceByChannel (Transformation|GetWorldLocation (Variables|/Script/MovementProject.FirstPersonCharacter|GetplayerCamera (Variables|Default|GetowningPlayer))) (+ (Transformation|GetWorldLocation (Variables|/Script/MovementProject.FirstPersonCharacter|GetplayerCamera (Variables|Default|GetowningPlayer))) (* (Math|Vector|GetForwardVector (Variables|/Script/MovementProject.FirstPersonCharacter|GetplayerCamera (Variables|Default|GetowningPlayer))) 1.5e+02)) 25.0 "TraceTypeQuery3" false (Utilities|Array|MakeArray (Variables|Default|GetowningPlayer)) "ForDuration"))
    (for _array_element _outhits
      (Game|Damage|ApplyDamage (.HitActor (Collision|BreakHitResult _array_element)) (Variables|Default|Getdamage) 0 0))
    (Utilities|FlowControl|Sequence
      (:then_0
        (if _returnvalue
          (Camera|PlayWorldCameraShake "/Game/Blueprints/Weapons/CameraShakes/Default_Shake.Default_Shake_C" (Transformation|GetWorldLocation (Variables|/Script/MovementProject.FirstPersonCharacter|GetplayerCamera (Variables|Default|GetowningPlayer))) 0.0 1e+01)))
      (:then_1
        (Utilities|FlowControl|Delay (Variables|Default|GetrateOfFire))
        (Variables|Default|SetcanAttack true)))))

(fn ConstructionScript
  (|CallParentFunction))