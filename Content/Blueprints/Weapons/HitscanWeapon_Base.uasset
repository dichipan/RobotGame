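; Base hitscan weapon Blueprint that fires instant line-trace shots from the owning player's camera.
; Attack checks ammo and a fire lock, spends a round, triggers recoil, then damages any actor hit by the trace, which ignores the owner and draws debug lines.
; A rate-of-fire delay releases the lock, and full-auto weapons re-call Attack while the player holds the attack input.
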(event EventAttack
  (params (player :type First%20Person%20Character%20Object%20Reference))
  (Variables|Default|SetowningPlayer player)
  (if (and (> (Variables|Default|GetammoMagazineCurrent) 0) (Variables|Default|GetcanAttack))
    (Math|Integer|DecrementInt (Variables|Default|GetammoMagazineCurrent)
      (:%20%20
        (CallFunction|Recoil)
        (Variables|Default|SetcanAttack false)
        (bind (_outhit _returnvalue) (Collision|LineTraceByChannel (Transformation|GetWorldLocation (Variables|/Script/MovementProject.FirstPersonCharacter|GetplayerCamera (Variables|Default|GetowningPlayer))) (+ (Transformation|GetWorldLocation (Variables|/Script/MovementProject.FirstPersonCharacter|GetplayerCamera (Variables|Default|GetowningPlayer))) (* (Math|Vector|GetForwardVector (Variables|/Script/MovementProject.FirstPersonCharacter|GetplayerCamera (Variables|Default|GetowningPlayer))) 5e+03)) "TraceTypeQuery3" false (Utilities|Array|MakeArray (Variables|Default|GetowningPlayer)) "ForDuration"))
        (Utilities|FlowControl|Sequence
          (:then_0
            (if _returnvalue
              (Game|Damage|ApplyDamage (.HitActor (Collision|BreakHitResult _outhit)) (Variables|Default|Getdamage) 0 0)))
          (:then_1
            (Utilities|FlowControl|Delay (Variables|Default|GetrateOfFire))
            (Variables|Default|SetcanAttack true)
            (if (and (Variables|/Script/MovementProject.FirstPersonCharacter|GetholdingAttack (Variables|Default|GetowningPlayer)) (Variables|Default|GetFullAuto?))
              (Class|Weapon|Attack (Variables|Default|GetowningPlayer)))))))))

(fn ConstructionScript
  (|CallParentFunction))