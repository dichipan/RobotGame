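; Base weapon Blueprint providing shared firing feedback and an empty-magazine reload check, with Attack and SecondaryAttack as debug-print placeholders.
; Recoil triggers Niagara, sound, optional arms montage, crosshair spread and camera shake, plus a weapon-slot kickback when not aiming, which also deactivates Niagara on finish.
; CameraRecoil uses timelines to add randomized pitch and yaw, then interpolate control rotation back toward the player's LookRotation.
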(event Custom|Recoil
  (bind _owningplayer (Variables|Default|GetowningPlayer))
  (bind _weaponslot (Variables|/Script/MovementProject.FirstPersonCharacter|GetweaponSlot _owningplayer))
  (bind _relativelocation (Variables|/Script/Engine.SceneComponent|GetRelativeLocation _weaponslot))
  (Components|Activation|Activate (Variables|Default|GetNiagara) false)
  (CallFunction|PlayAnimation)
  (CallFunction|StartImpactTimeline)
  (CallFunction|CameraRecoil)
  (Camera|PlayWorldCameraShake "/Game/Blueprints/Weapons/CameraShakes/Default_Shake.Default_Shake_C" (Transformation|GetWorldLocation (Variables|/Script/MovementProject.FirstPersonCharacter|GetplayerCamera (Variables|Default|GetowningPlayer))) 0.0 1e+01)
  (if (not (Variables|/Script/MovementProject.FirstPersonCharacter|GetisAiming (Variables|Default|GetowningPlayer)))
    (bind _newtrack_0 (Timeline|Timeline PlayFromStart)
      (:Update
        (Transformation|SetRelativeLocation _weaponslot (Math|Vector|MakeVector (Math|Float|Clamp(Float) (+ (.x _relativelocation) (Math|Float|Lerp 0.0 -1.0 _newtrack_0)) -9.0 0.0) (.y _relativelocation) (.z _relativelocation)) false false))
      (:Finished
        (Components|Activation|Deactivate (Variables|Default|GetNiagara))))))

(event Custom|PlayAnimation
  (Audio|PlaySoundatLocation "/Game/Assets/Audio/GunModulator.GunModulator" (Transformation|GetActorLocation) "0, 0, 0" 1.0 1.0 0.0 "/Game/Assets/Audio/GunSoundAttenuation.GunSoundAttenuation" 0 0 0)
  (if (Variables|Default|GetAnimationImplemented?)
    (Animation|Montage|PlayMontage (Variables|/Game/Blueprints/Player/FirstPersonCharacter_Base.FirstPersonCharacter_Base_C|GetArms (.AsFirst%20Person%20Character%20Base (Utilities|Casting|CastToFirstPersonCharacter_Base (Variables|Default|GetowningPlayer)))) "/Game/Assets/Arms/Anims/Arms_Anim_PistolShoot_Montage.Arms_Anim_PistolShoot_Montage" 1.0 0.0 "Attack")))

(event Custom|SecondaryAttack
  (params (Player :type First%20Person%20Character%20Base%20Object%20Reference))
  (Development|PrintString "second"))

(event Custom|StartImpactTimeline
  (bind _newtrack_0 (Timeline|ImpactTimeline PlayFromStart)
    (:Update
      (Variables|Default|SetcrosshairAmountCurrent (Math|Float|Lerp 0.0 (Variables|Default|GetcrosshairAmountMax) _newtrack_0)))))

(event Custom|CameraRecoil
  (bind _owningplayer (Variables|Default|GetowningPlayer))
  (CallFunction|StopRecoilDown)
  (Variables|Default|SetRandomHorizontalRecoil (Math|Random|RandomFloatinRange (Variables|Default|GethorizontalRecoilBottom) (Variables|Default|GethorizontalRecoilTop)))
  (Variables|Default|SetRandomVerticalRecoil (Math|Random|RandomFloatinRange (Variables|Default|GetverticalRecoilBottom) (Variables|Default|GetverticalRecoilTop)))
  (Audio|Components|Audio|Stop (Variables|Default|GetRecoilDown))
  (bind _newtrack_0 (Timeline|RecoilUp PlayFromStart)
    (:Update
      (Pawn|Input|AddControllerPitchInput (Variables|Default|GetowningPlayer) (* (* (* (- _newtrack_0 (Variables|Default|GetLerpValue)) (Utilities|Time|GetWorldDeltaSeconds)) -1.0) (Variables|Default|GetRandomVerticalRecoil)))
      (Pawn|Input|AddControllerYawInput (Variables|Default|GetowningPlayer) (* (* (* (- _newtrack_0 (Variables|Default|GetLerpValue)) (Utilities|Time|GetWorldDeltaSeconds)) -1.0) (Variables|Default|GetRandomHorizontalRecoil)))
      (Variables|Default|SetLerpValue (* (- _newtrack_0 (Variables|Default|GetLerpValue)) (Utilities|Time|GetWorldDeltaSeconds))))
    (:Finished
      (Variables|Default|SetLerpValue 0.0)
      (Variables|Default|SetNewControlRot (Pawn|GetControlRotation (Variables|Default|GetowningPlayer) :!class /Script/Engine.Pawn))
      (bind _newtrack_0_2 (Timeline|RecoilDown PlayFromStart)
        (:Update
          (Pawn|SetControlRotation (Pawn|GetController _owningplayer) (Math|Interpolation|RInterpTo (Variables|Default|GetNewControlRot) (Variables|/Script/MovementProject.FirstPersonCharacter|GetlookRotation _owningplayer) _newtrack_0_2 1.0)))))))

(event Custom|StopRecoilDown
  (bind _owningplayer (Variables|Default|GetowningPlayer))
  (if (Audio|Components|Audio|IsPlaying (Variables|Default|GetRecoilDown))
    (bind _newtrack_0 (Timeline|RecoilDown Stop)
      (:Update
        (Pawn|SetControlRotation (Pawn|GetController _owningplayer) (Math|Interpolation|RInterpTo (Variables|Default|GetNewControlRot) (Variables|/Script/MovementProject.FirstPersonCharacter|GetlookRotation _owningplayer) _newtrack_0 1.0))))))

(event Custom|ReloadCheck
  (if (<= (Variables|Default|GetammoMagazineCurrent) 0)
    (Class|Weapon|Reload)))

(event EventAttack
  (params (player :type First%20Person%20Character%20Object%20Reference))
  (Development|PrintString (Utilities|String|Append "Hello, " (Utilities|GetDisplayName player))))

(fn ConstructionScript)