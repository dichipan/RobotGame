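; Sliding door Blueprint that raises its mesh along Z when interacted with, provided it is unlocked.
; A FlipFlop toggles the DoorMove timeline between play and reverse, while a DoorClose timeline acts as an auto-close timer that manual closing stops.
; Activate unlocks the door and swaps its material.
; The first interaction also fires every linked Trigger with the player, even if the door is locked.
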(event Custom|UnlockDoor
  (Variables|Default|SetCanOpen? true)
  (Rendering|Material|SetMaterial (Variables|Default|GetDoor) 0 "/Game/Blueprints/Pickups/Health_Mat.Health_Mat"))

(event Custom|DoorSwitch
  (Utilities|FlowControl|FlipFlop
    (:A
      (Variables|Default|SetDoorOpen true)
      (bind _newtrack_0 (Timeline|DoorMove Play)
        (:Update
          (Transformation|SetRelativeLocation (Variables|Default|GetDoor) (Math|Vector|MakeVector 0.0 0.0 (Math|Float|Lerp 0.0 2.5e+02 _newtrack_0)) false false))
        (:Finished
          (if (Variables|Default|GetDoorOpen)
            (Timeline|DoorClose PlayFromStart
              (:Finished
                (CallFunction|DoorSwitch)))))))
    (:B
      (Utilities|FlowControl|Sequence
        (:then_0
          (Variables|Default|SetDoorOpen false)
          (Timeline|DoorMove Reverse))
        (:then_1
          (Timeline|DoorClose Stop))))))

(event EventActivate
  (params (Player :type First%20Person%20Character%20Base%20Object%20Reference))
  (CallFunction|UnlockDoor))

(event EventInteract
  (params (Player :type First%20Person%20Character%20Base%20Object%20Reference))
  (Utilities|FlowControl|Sequence
    (:then_0
      (if (Variables|Default|GetCanOpen?)
        (CallFunction|DoorSwitch)))
    (:then_1
      (Utilities|FlowControl|DoOnce false
        (:Completed
          (for _array_element (Variables|Default|GetTriggers)
            (Default|Trigger _array_element Player)))))))

(fn ConstructionScript
  (|CallParentFunction))