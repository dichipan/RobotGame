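; Base key pickup that unlocks a set of linked doors when the player touches it.
; On overlap with a player-controlled FirstPersonCharacter_Base, it calls ActivateMessage on each entry in UnlockedDoors, passing the character, then destroys itself.
; A hardcoded "BLUE DOORS UNLOCKED" string prints on every overlap, before the player check runs.
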(event Collision|EventActorBeginOverlap
  (params (OtherActor :type Actor%20Object%20Reference))
  (bind _asfirst_person_character_base (Utilities|Casting|CastToFirstPersonCharacter_Base OtherActor))
  (Development|PrintString "BLUE DOORS UNLOCKED")
  (if (and (Utilities|ClassIsChildOf (Utilities|GetClass OtherActor) "/Game/Blueprints/Player/FirstPersonCharacter_Base.FirstPersonCharacter_Base_C") (Pawn|IsPlayerControlled _asfirst_person_character_base))
    (for _array_element (Variables|Default|GetUnlockedDoors)
      (Class|ActivateInterface|Activate(Message) _array_element _asfirst_person_character_base))
    (Actor|DestroyActor)))

(fn ConstructionScript
  (|CallParentFunction))