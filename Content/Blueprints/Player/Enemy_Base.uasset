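; Enemy base character that fights the player using a randomized event-driven AI loop, started by TriggerAI.
; After random delays, RandomSelection favors attacking over briefly moving toward the player, and each action loops back into selection.
; Attacks require a camera-to-camera line trace, then fire the child-actor Weapon_Base while the FollowPlayer timeline keeps yaw on the player.
; Without line of sight, it moves to a random reachable nearby point before choosing again.
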(event Custom|Look%20At%20Player
  (Transformation|SetActorRotation (Math|Rotator|MakeRotator 0.0 0.0 (.yaw (Math|Rotator|FindLookatRotation (Transformation|GetActorLocation) (Transformation|GetActorLocation (Game|Player|GetPlayerPawn 0)))))))

(event Custom|Attack%20Player
  (CallFunction|LookatPlayer)
  (Variables|Default|SetholdingAttack true)
  (bind _playervisible_ (CallFunction|LineOfSightCheck))
  (if _playervisible_
    (Class|Weapon|Attack (.AsWeapon%20Base (Utilities|Casting|CastToWeapon_Base (Variables|/Script/Engine.ChildActorComponent|GetChildActor (Variables|Default|GetWeapon)))) self)
    (Timeline|FollowPlayer PlayFromStart
      (:Update
        (CallFunction|LookatPlayer))
      (:Finished
        (Variables|Default|SetholdingAttack false)
        (CallFunction|RandomSelection)))
    (else
      (CallFunction|MoveRandomLocation))))

(event Custom|MoveRandomLocation
  (AI|AIMoveTo (Pawn|GetControlledPawn (Pawn|GetController)) (.RandomLocation (AI|Navigation|GetRandomReachablePointinRadius (Transformation|GetActorLocation) 1e+03 0 0)) 0 5.0 false
    (:OnSuccess
      _)
    (:OnFail
      _))
  (Utilities|FlowControl|Delay 0.1)
  (CallFunction|LookatPlayer)
  (CallFunction|RandomSelection))

(event Custom|RandomSelection
  (Utilities|FlowControl|Delay (Math|Random|RandomFloatinRange 0.0 2.0))
  (switch int (Math|Random|RandomIntegerinRange 0 5)
    (:0
      (CallFunction|AttackPlayer :!label _label))
    (:1
      (CallFunction|MoveTowardsPlayer :!label _label_2))
    (:2
      (goto _label))
    (:3
      (goto _label))
    (:4
      (goto _label_2))
    (:5
      (goto _label))))

(event Custom|MoveTowardsPlayer
  (Utilities|FlowControl|Sequence
    (:then_0
      (AI|AIMoveTo (Pawn|GetControlledPawn (Pawn|GetController)) "0, 0, 0" (Game|Player|GetPlayerPawn 0) 5.0 false))
    (:then_1
      (Utilities|FlowControl|Delay (Math|Random|RandomFloatinRange 0.1 3.0))
      (Components|Movement|StopMovementImmediately (Variables|Character|GetCharacterMovement))
      (CallFunction|RandomSelection))))

(event Custom|TriggerEnemy
  (Utilities|FlowControl|Delay 1.0)
  (CallFunction|RandomSelection))

(event EventTriggerAI
  (CallFunction|TriggerEnemy))

(fn ConstructionScript
  (|CallParentFunction))

(fn LineOfSightCheck
  (bind _outhit (Collision|LineTraceByChannel (Transformation|GetWorldLocation (Variables|Default|GetplayerCamera)) (Transformation|GetWorldLocation (Variables|/Script/MovementProject.FirstPersonCharacter|GetplayerCamera (.AsFirst%20Person%20Character%20Base (Utilities|Casting|CastToFirstPersonCharacter_Base (Game|Player|GetPlayerPawn 0))))) "TraceTypeQuery1" false (Utilities|Array|MakeArray self) "ForDuration"))
  (return (== (.HitActor (Collision|BreakHitResult _outhit)) (Game|GetPlayerCharacter 0))))