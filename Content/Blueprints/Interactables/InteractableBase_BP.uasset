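; Base Blueprint for interactable objects that players use by spending points.
; Hint copies the object's hint text to the player, while Interact calls SpendPoints, which deducts the point cost only if the player can afford it.
; A successful payment triggers InteractAction, a placeholder for child classes to override that only prints a not-implemented message here.
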(event Custom|InteractAction
  (params (Player :type First%20Person%20Character%20Base%20Object%20Reference))
  (Development|PrintString "InteractAction not implemented"))

(event EventBeginPlay)

(event Collision|EventActorBeginOverlap
  (params (OtherActor :type Actor%20Object%20Reference)))

(event EventHint
  (params (Player :type First%20Person%20Character%20Base%20Object%20Reference))
  (Variables|/Game/Blueprints/Player/FirstPersonCharacter_Base.FirstPersonCharacter_Base_C|SetHint Player (Variables|Default|GetHintText)))

(event EventInteract
  (params (Player :type First%20Person%20Character%20Base%20Object%20Reference))
  (bind _enoughpoints_ (CallFunction|SpendPoints Player))
  (if _enoughpoints_
    (CallFunction|InteractAction Player)))

(fn ConstructionScript)

(fn SpendPoints
  (params (Player :type First%20Person%20Character%20Base%20Object%20Reference))
  (if (>= (Variables|/Script/MovementProject.FirstPersonCharacter|Getpoints Player) (Variables|Default|GetPointCost))
    (Class|FirstPersonCharacter|AddPoints Player (* (Variables|Default|GetPointCost) -1))
    (return true)
    (else
      (return false))))