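; Interactable weapon pickup Blueprint that gives its configured weapon class to the player who interacts with it.
; InteractAction stores the player and branches on how many weapons they carry.
; With one or none, it adds the weapon and switches to index 1.
; With more, it only sets the class of the player's Weapon child actor component, leaving the weapons list untouched.
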(event Custom|Add%20Weapon
  (Default|AddWeapon (Variables|Default|GetPlayer) (Variables|Default|GetWeapon))
  (Default|SwitchWeapon (Variables|Default|GetPlayer) 1))

(event Custom|ChangeWeapon
  (ChildActorComponent|SetChildActorClass (Variables|/Game/Blueprints/Player/FirstPersonCharacter_Base.FirstPersonCharacter_Base_C|GetWeapon (Variables|Default|GetPlayer)) (Variables|Default|GetWeapon)))

(event EventInteractAction
  (params (Player :type First%20Person%20Character%20Base%20Object%20Reference))
  (Variables|Default|SetPlayer Player)
  (if (> (Utilities|Array|Length (Variables|/Game/Blueprints/Player/FirstPersonCharacter_Base.FirstPersonCharacter_Base_C|GetWeapons (Variables|Default|GetPlayer))) 1)
    (CallFunction|ChangeWeapon)
    (else
      (CallFunction|AddWeapon))))

(fn ConstructionScript
  (|CallParentFunction))