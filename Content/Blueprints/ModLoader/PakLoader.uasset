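; PakLoader is a test Blueprint that mounts a pak of external content at runtime in packaged builds.
; On BeginPlay it checks and mounts the pak at PakPath, registers the /Hello/ mount point, lists that directory's files and plays the Water sound from it.
; Each step prints debug output, and validation is only printed, not enforced.
; Disconnected nodes for listing pak contents and loading its asset registry never run.
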(event EventBeginPlay
  (bind _pakpath (Variables|Default|GetPakPath))
  (if (Class|PakLoaderLibrary|IsPackagedBuild)
    (bind _returnvalue (Class|PakLoaderLibrary|IsValidPakFile _pakpath))
    (Development|PrintString (Utilities|String|Append _pakpath " " (Utilities|String|ToString(Boolean) _returnvalue)))
    (bind _returnvalue_2 (Class|PakLoaderLibrary|MountPakFile (Variables|Default|GetPakPath) "../../../"))
    (Development|PrintString (Utilities|String|Append (Utilities|String|ToString(Boolean) _returnvalue_2) " mounted"))
    (Class|PakLoaderLibrary|RegisterMountPoint "/Hello/" "../../../Hello/Content/")
    (bind _returnvalue_3 (Class|PakLoaderLibrary|GetFilesinPakDirectory "../../../Hello/" true))
    (for _array_element _returnvalue_3
      (Development|PrintString _array_element))
    (Audio|PlaySound2D (Class|PakLoaderLibrary|GetPakFileSound "/Hello/Audio/Water") 1.0 1.0 0.0 0 0)))

(fn ConstructionScript)