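; Base enemy Blueprint that moves to its Spawner's location after spawning, then endlessly chases the first-person player through looping AI MoveTo calls.
; Damage lowers Health and awards the attacking player points, with more for a kill, before Death and actor destruction at zero.
; Attack, not called within this graph, plays a robot montage, then after a delay runs a debug-drawn forward line trace to damage the player.
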(event EventBeginPlay
  (|CallParentFunction)
  (Utilities|FlowControl|Delay 0.2)
  (Utilities|FlowControl|Sequence
    (:then_0
      (AI|AIMoveTo (Pawn|GetControlledPawn (Pawn|GetController)) (Transformation|GetActorLocation (Variables|Default|Getspawner)) 0 5.0 false
        (:OnSuccess
          _)
        (:OnFail
          _))
      (Class|EnemyBase|ChasePlayer))
    (:then_1
      (bind _returnvalue (Actor|GetActorOfClass "/Game/Blueprints/Player/FirstPersonCharacter_Base.FirstPersonCharacter_Base_C"))
      (Variables|Default|SettargetPlayer _returnvalue))))

(event EventChasePlayer
  (AI|AIMoveTo (Pawn|GetControlledPawn (Pawn|GetController)) "0, 0, 0" (Variables|Default|GettargetPlayer) 5.0 false
    (:OnSuccess
      _)
    (:OnFail
      _))
  (Class|EnemyBase|ChasePlayer))

(event EventAttack
  (bind _capsulecomponent (Variables|Default|GetCapsuleComponent))
  (bind _returnvalue (Transformation|GetWorldLocation _capsulecomponent))
  (Animation|Montage|PlayMontage (Variables|Character|GetMesh) "/Game/Assets/NewerRobot/Animations/importfolder/RobotMontage.RobotMontage" 1.0 0.0 "Attack1"
    (:then
      (Utilities|FlowControl|Delay 0.6)
      (bind _outhit (Collision|LineTraceByChannel _returnvalue (+ _returnvalue (* (Math|Vector|GetForwardVector _capsulecomponent) (Variables|Default|GetattackDistance))) "TraceTypeQuery1" false 0 "ForDuration"))
      (if (Utilities|ClassIsChildOf (Utilities|GetClass (.HitActor (Collision|BreakHitResult _outhit))) "/Game/Blueprints/Player/FirstPersonCharacter_Base.FirstPersonCharacter_Base_C")
        (Game|Damage|ApplyDamage (.HitActor (Collision|BreakHitResult _outhit)) (Variables|Default|Getdamage) 0 0)))))

(event Game|Damage|EventAnyDamage
  (params (Damage :type Float%20%28single-precision%29) (DamageType :type Damage%20Type%20Object%20Reference) (InstigatedBy :type Controller%20Object%20Reference) (DamageCauser :type Actor%20Object%20Reference))
  (bind _output_get (Variables|Default|Sethealth (- (Variables|Default|Gethealth) Damage)))
  (CallFunction|AddPointstoPlayer DamageCauser)
  (if (<= _output_get 0.0)
    (Class|EnemyBase|Death)
    (Actor|DestroyActor)))

(fn ConstructionScript)

(fn AddPointstoPlayer
  (params (Player :type Actor%20Object%20Reference))
  (bind _asfirst_person_character_base (Utilities|Casting|CastToFirstPersonCharacter_Base Player))
  (Utilities|IsValid _asfirst_person_character_base
    (:Is%20Valid
      (if (<= (Variables|Default|Gethealth) 0.0)
        (Class|FirstPersonCharacter|AddPoints _asfirst_person_character_base 50)
        (else
          (Class|FirstPersonCharacter|AddPoints _asfirst_person_character_base 10)))
      (Development|PrintString (Utilities|String|ToString(Integer) (Variables|/Script/MovementProject.FirstPersonCharacter|Getpoints _asfirst_person_character_base))))))